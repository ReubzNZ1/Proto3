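; BP_Spook is an enemy that can open doors it is near.
; It stores a local door reference when given one and tells its AI controller it is near a door, reversing both when cleared.
; SpookOpenDoor opens the stored door, then clears the reference and the near-door state.
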(event `self.ReceiveBeginPlay`)

(event `UpdateLocalDoor`
  (params (Door :type "/Game/Blueprints/BP_Door Object Reference"))
  ;[1 1 1] Update local door
  (set `self.LocalDoor` Door)
  (message `/Game/Enemy/I_SpookNearDoor.UpdateNearDoor` (`AIBlueprintHelperLibrary.GetAIController` self) true))

(event `ClearLocalDoor`
  ;[1 1 1] Clear local door
  (set `self.LocalDoor` null)
  (message `/Game/Enemy/I_SpookNearDoor.UpdateNearDoor` (`AIBlueprintHelperLibrary.GetAIController` self) false))

(event `/Game/Enemy/I_OpenDoor.SpookOpenDoor`
  ;[1 1 1] Open door
  (`/Game/Blueprints/BP_Door.Open Door` (`self.LocalDoor`))
  (`self.ClearLocalDoor`))

(fn `UserConstructionScript`)