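; BP_ParentLockedDoor is a parent Blueprint for locked doors that tracks whether the player holds the key needed to unlock it.
; BeginPlay sets a default key name and marks the door locked.
; While locked, Tick polls the first-person character's KeysObtained list and sets Unlocked when an entry matches KeyToUnlock.
; It contains no door movement or other response to unlocking, only the state flag.
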(event `self.ReceiveBeginPlay`
  (`parent.ReceiveBeginPlay`)
  (set `self.KeyToUnlock` "Default")
  (set `self.Unlocked` false))

(event `self.ReceiveTick`
  (params (DeltaSeconds :type "Float (single-precision)"))
  (`parent.ReceiveTick` DeltaSeconds)
  (if (not (`self.Unlocked`))
    (bind _asbp_first_person_character (cast `/Game/Blueprints/BP_FirstPersonCharacter` (`GameplayStatics.GetPlayerCharacter` 0)))
    (for _array_element (`/Game/Blueprints/BP_FirstPersonCharacter.KeysObtained` _asbp_first_person_character)
      (if (`KismetStringLibrary.EqualEqual_StrStr` (`self.KeyToUnlock`) _array_element)
        (set `self.Unlocked` true)))))

(fn `UserConstructionScript`
  (`parent.UserConstructionScript`))