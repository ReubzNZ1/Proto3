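; BP_DefaultKey is a base key pickup that the first-person character collects by interacting while in range.
; Overlap events track range, and Tick polls the player's Interacting flag until the key is picked up.
; Pickup hides the model, ignores its collision, zeroes the light intensity limit, adds KeyName to the player's KeysObtained and plays a one-time sound.
; BeginPlay sets a placeholder name and an empty sound.
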(event `self.ReceiveBeginPlay`
  (set `self.KeyName` "Default")
  (set `self.SoundEffect` null))

(event `self.ReceiveActorBeginOverlap`
  (params (OtherActor :type "Actor Object Reference"))
  (`parent.ReceiveActorBeginOverlap` null)
  (if (== (`GameplayStatics.GetObjectClass` OtherActor) "/Game/Blueprints/BP_FirstPersonCharacter.BP_FirstPersonCharacter_C")
    (set `self.InRange` true)))

(event `self.ReceiveActorEndOverlap`
  (params (OtherActor :type "Actor Object Reference"))
  (if (== (`GameplayStatics.GetObjectClass` OtherActor) "/Game/Blueprints/BP_FirstPersonCharacter.BP_FirstPersonCharacter_C")
    (set `self.InRange` false)))

(event `self.ReceiveTick`
  (params (DeltaSeconds :type "Float (single-precision)"))
  (`parent.ReceiveTick` DeltaSeconds)
  (if (`self.IsPickedUp`)
    _
    (elif (`self.InRange`)
      (bind _asbp_first_person_character (cast `/Game/Blueprints/BP_FirstPersonCharacter` (`GameplayStatics.GetPlayerCharacter` 0)))
      (if (`/Game/Blueprints/BP_FirstPersonCharacter.bInteracting` _asbp_first_person_character)
        (set `self.IsPickedUp` true)
        (`SceneComponent.SetVisibility` (`self.Model`) false false)
        (`PrimitiveComponent.SetCollisionResponseToAllChannels` (`self.Model`) "ECR_Ignore")
        (set `self.MaxLightIntensity` 0.0)
        (`KismetArrayLibrary.Array_AddUnique` (`/Game/Blueprints/BP_FirstPersonCharacter.KeysObtained` _asbp_first_person_character) (`self.KeyName`))
        (`/Engine/EditorBlueprintResources/StandardMacros.DoOnce` false
          (:`Completed`
            (`GameplayStatics.PlaySound2D` (`self.SoundEffect`) 1.0 1.0 0.0 null null)))))))

(fn `UserConstructionScript`
  (`parent.UserConstructionScript`))