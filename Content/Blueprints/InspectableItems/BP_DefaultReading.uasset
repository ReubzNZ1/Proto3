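; Base-style readable inspectable actor that shows a text string on the player's UI while the player holds interact nearby.
; Overlap with BP_FirstPersonCharacter sets an in-range flag, and leaving clears it and hides the text.
; While in range, Tick polls the character's Interacting state each frame to show or clear the text on WBP_PlayerUI.
; BeginPlay fills the display string with placeholder text.
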(event `self.ReceiveBeginPlay`
  (`parent.ReceiveBeginPlay`)
  (set `self.sTextToDisplay` "This is some weird placeholder text \nIgnore me and replace later \nI'm being serious, ignore this"))

(event `self.ReceiveActorBeginOverlap`
  (params (OtherActor :type "Actor Object Reference"))
  (`parent.ReceiveActorBeginOverlap` null)
  (if (== (`GameplayStatics.GetObjectClass` OtherActor) "/Game/Blueprints/BP_FirstPersonCharacter.BP_FirstPersonCharacter_C")
    (set `self.bInRange` true)))

(event `self.ReceiveActorEndOverlap`
  (params (OtherActor :type "Actor Object Reference"))
  (if (== (`GameplayStatics.GetObjectClass` OtherActor) "/Game/Blueprints/BP_FirstPersonCharacter.BP_FirstPersonCharacter_C")
    (set `self.bInRange` false)
    (bind _aswbp_player_ui (cast `/Game/Blueprints/Widgets/WBP_PlayerUI` (`/Game/Blueprints/BP_FirstPersonCharacter.PlayerUI` (stale `self.ReceiveTick` _asbp_first_person_character))))
    (`/Game/Blueprints/Widgets/WBP_PlayerUI.SetOnScreenText` _aswbp_player_ui "")
    (set `/Game/Blueprints/Widgets/WBP_PlayerUI.bIsTextVisible` false _aswbp_player_ui)))

(event `self.ReceiveTick`
  (params (DeltaSeconds :type "Float (single-precision)"))
  (`parent.ReceiveTick` DeltaSeconds)
  (if (`self.bInRange`)
    (bind _asbp_first_person_character (cast `/Game/Blueprints/BP_FirstPersonCharacter` (`GameplayStatics.GetPlayerCharacter` 0)))
    (if (`/Game/Blueprints/BP_FirstPersonCharacter.bInteracting` _asbp_first_person_character)
      (bind _playerui (`/Game/Blueprints/BP_FirstPersonCharacter.PlayerUI` _asbp_first_person_character))
      (bind _aswbp_player_ui (cast `/Game/Blueprints/Widgets/WBP_PlayerUI` _playerui))
      (`/Game/Blueprints/Widgets/WBP_PlayerUI.SetOnScreenText` _aswbp_player_ui (`self.sTextToDisplay`))
      (set `/Game/Blueprints/Widgets/WBP_PlayerUI.bIsTextVisible` true _aswbp_player_ui)
      (else
        (bind _aswbp_player_ui_2 (cast `/Game/Blueprints/Widgets/WBP_PlayerUI` _playerui))
        (`/Game/Blueprints/Widgets/WBP_PlayerUI.SetOnScreenText` _aswbp_player_ui_2 "")
        (set `/Game/Blueprints/Widgets/WBP_PlayerUI.bIsTextVisible` false _aswbp_player_ui_2)))))

(fn `UserConstructionScript`
  (`parent.UserConstructionScript`))