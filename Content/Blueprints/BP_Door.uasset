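; BP_Door is a lockable swinging door that registers itself with BP_Spook while that actor overlaps its Box.
; When Unlocked, OpenDoor and SpookOpenDoorReverse use separate FlipFlops and timelines to swing it 90 degrees in opposite directions or back.
; Tick switches the door's collision object type by lock state.
; OpenDoor toggles Open on every timeline update, and an unconnected duplicate swing chain never runs.
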(event `self.ReceiveBeginPlay`)

(event `self.ReceiveTick`
  (params (DeltaSeconds :type "Float (single-precision)"))
  (if (`self.Unlocked`)
    (`PrimitiveComponent.SetCollisionObjectType` (`self.Door`) "ECC_GameTraceChannel2")
    (else
      (`PrimitiveComponent.SetCollisionObjectType` (`self.Door`) "ECC_WorldDynamic"))))

(event `Open Door`
  (if (`self.Unlocked`)
    ;[1 0 0.4644] Door Animation Event
    (`/Engine/EditorBlueprintResources/StandardMacros.FlipFlop`
      (:`A`
        (bind (_direction _doorfloat) (`Timeline|OpenDoor` :!label _label)
          (:`Update`
            (`SceneComponent.K2_SetRelativeRotation` (`self.Door`) (`KismetMathLibrary.MakeRotator` 0.0 0.0 (`KismetMathLibrary.Lerp` 0.0 90.0 _doorfloat)) false false)
            (if (`self.Open`)
              (set `self.Open` false)
              (else
                (set `self.Open` true))))))
      (:`B`
        (goto _label :!via `Reverse`)))))

(event `self.Box.OnComponentBeginOverlap`
  (params (OverlappedComponent :type "PrimitiveComponent Object Reference") (OtherActor :type "Actor Object Reference") (OtherComp :type "PrimitiveComponent Object Reference") (OtherBodyIndex :type Integer) (bFromSweep :type Boolean) (SweepResult :type "HitResult Structure (by ref)"))
  ;[1 1 1] Spook is overlapping
  (bind _asbp_spook (cast `/Game/Enemy/BP_Spook` OtherActor))
  (`/Game/Enemy/BP_Spook.UpdateLocalDoor` _asbp_spook self))

(event `SpookOpenDoorReverse`
  (if (`self.Unlocked`)
    (`/Engine/EditorBlueprintResources/StandardMacros.FlipFlop`
      (:`A`
        (bind (_direction _doorfloat) (`Timeline|Timeline_0` :!label _label_2)
          (:`Update`
            (`SceneComponent.K2_SetRelativeRotation` (`self.Door`) (`KismetMathLibrary.MakeRotator` 0.0 0.0 (`KismetMathLibrary.Lerp` 0.0 -90.0 _doorfloat)) false false))))
      (:`B`
        (goto _label_2 :!via `Reverse`)))))

(event `self.Box.OnComponentEndOverlap`
  (params (OverlappedComponent :type "PrimitiveComponent Object Reference") (OtherActor :type "Actor Object Reference") (OtherComp :type "PrimitiveComponent Object Reference") (OtherBodyIndex :type Integer))
  ;[1 1 1] Spook is gone
  (bind _asbp_spook (cast `/Game/Enemy/BP_Spook` OtherActor))
  (`/Game/Enemy/BP_Spook.ClearLocalDoor` _asbp_spook))

(fn `UserConstructionScript`)