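; BP_Heartbeat is a proximity fear-audio actor that plays heartbeat and fast breathing when a BP_Spook comes near the player.
; Each Tick it moves its root to the player character's mesh, carrying its detection Sphere along.
; Sphere overlap with a BP_Spook activates both sounds, which start inactive.
; On exit the Audio component stops, while breathing switches to a fade-out sound, never switched back, then deactivates after a delay.
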(event `self.ReceiveBeginPlay`
  (`ActorComponent.SetActive` (`self.Audio`) false false)
  (`ActorComponent.SetActive` (`self.Fastbreathing`) false false))

(event `self.ReceiveTick`
  (params (DeltaSeconds :type "Float (single-precision)"))
  (`SceneComponent.K2_SetWorldLocation` (`self.DefaultSceneRoot`) (`SceneComponent.K2_GetComponentLocation` (`Character.Mesh` (`GameplayStatics.GetPlayerCharacter` 0))) false false))

(event `self.Sphere.OnComponentBeginOverlap`
  (params (OverlappedComponent :type "PrimitiveComponent Object Reference") (OtherActor :type "Actor Object Reference") (OtherComp :type "PrimitiveComponent Object Reference") (OtherBodyIndex :type Integer) (bFromSweep :type Boolean) (SweepResult :type "HitResult Structure (by ref)"))
  (cast `/Game/Enemy/BP_Spook` OtherActor)
  (`ActorComponent.SetActive` (`self.Audio`) true false)
  (`ActorComponent.SetActive` (`self.Fastbreathing`) true false))

(event `self.Sphere.OnComponentEndOverlap`
  (params (OverlappedComponent :type "PrimitiveComponent Object Reference") (OtherActor :type "Actor Object Reference") (OtherComp :type "PrimitiveComponent Object Reference") (OtherBodyIndex :type Integer))
  (cast `/Game/Enemy/BP_Spook` OtherActor)
  (`ActorComponent.SetActive` (`self.Audio`) false false)
  (`AudioComponent.SetSound` (`self.Fastbreathing`) "/Game/Assets/SFX/Player/BreathingHardFadeOut.BreathingHardFadeOut")
  (`KismetSystemLibrary.Delay` 4.0)
  (`ActorComponent.SetActive` (`self.Fastbreathing`) false true))

(fn `UserConstructionScript`)